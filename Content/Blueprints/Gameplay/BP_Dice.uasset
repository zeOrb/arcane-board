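; BP_Dice is a short-lived visual die that pops up, shows face Val to the camera and destroys itself.
; On BeginPlay, a timeline scaled by animation speed grows and lifts it, pauses briefly, then reverses.
; Rotation blends from a random rotator, re-rolled each update for a tumbling look, to the Orientation entry for Val, rotated into a camera-facing basis.
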(event EventBeginPlay
  (bind _returnvalue (Transformation|GetActorLocation))
  (bind _returnvalue_2 (Game|GetPlayerCameraManager 0))
  (bind _val (Variables|Default|GetVal))
  (bind _orientation (Variables|Default|GetOrientation))
  (bind _returnvalue_3 (Camera|GetCameraLocation _returnvalue_2))
  (bind _returnvalue_4 (- _val 1))
  (bind _returnvalue_5 (Math|Rotator|FindLookatRotation _returnvalue _returnvalue_3))
  (bind _output (Utilities|Array|Get(acopy) _orientation _returnvalue_4))
  (bind _returnvalue_6 (Math|Vector|GetRightVector _returnvalue_5))
  (bind _returnvalue_7 (Math|Vector|GetForwardVector _returnvalue_5))
  (bind _returnvalue_8 (Math|Vector|GetUpVector _returnvalue_5))
  (bind _returnvalue_9 (Math|Vector|NegateVector _returnvalue_8))
  (bind _returnvalue_10 (Math|Vector|NegateVector _returnvalue_7))
  (bind _returnvalue_11 (Math|Rotator|MakeRotationfromAxes _returnvalue_9 _returnvalue_6 _returnvalue_10))
  (Components|Timeline|SetPlayRate (Variables|Default|GetTimeline_0) (CallFunction|GetAnimationSpeed))
  (Variables|Default|SetOrigin (Transformation|GetActorLocation))
  (bind (_direction _newtrack_0) (Timeline|Timeline_0 PlayFromStart)
    (:Update
      (Transformation|SetActorScale3D (Math|Vector|Lerp(Vector) "0, 0, 0" "0.040000,0.040000,0.040000" _newtrack_0))
      (Transformation|SetActorLocation (Math|Vector|Lerp(Vector) (Variables|Default|GetOrigin) (+ (Variables|Default|GetOrigin) "0, 0,38.000000") _newtrack_0) false false)
      (Transformation|SetActorRotation (Math|Rotator|Lerp(Rotator) (Math|Random|RandomRotator true) (Math|Rotator|MakeRotationfromAxes (Math|Vector|RotateVector (Math|Vector|GetForwardVector _output) _returnvalue_11) (Math|Vector|RotateVector (Math|Vector|GetRightVector _output) _returnvalue_11) (Math|Vector|RotateVector (Math|Vector|GetUpVector _output) _returnvalue_11)) _newtrack_0)))
    (:Finished
      (if (Utilities|Enum|Equal(Enum) _direction "Forward")
        (Utilities|FlowControl|Delay 0.3)
        (Timeline|Timeline_0 ReverseFromEnd)
        (else
          (Actor|DestroyActor))))))

(event Collision|EventActorBeginOverlap
  (params (OtherActor :type Actor%20Object%20Reference)))

(event EventTick
  (params (DeltaSeconds :type Float%20%28single-precision%29)))

(fn ConstructionScript)