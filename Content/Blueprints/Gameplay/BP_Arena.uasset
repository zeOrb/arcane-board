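; Grid-based combat arena that builds an instanced tile floor and plays out unit actions and dice rolls.
; Construction lays the floor, BeginPlay adds cell instances, and movement-range events swap cells between two instanced meshes via sphere-overlap lookup.
; Move and move-attack actions attach units to spawned dummy actors, which timelines lerp with a height offset before reporting completion.
; Spawned dice face the camera and advance the combat engine's initiative state when destroyed.
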(event Custom|OnDiceFinished
  (params (DestroyedActor :type Actor%20Object%20Reference))
  (Class|CombatEngine|UpdateState (Class|Arena|GetCombatEngine) "EInitiativeRoll"))

(event EventBeginPlay
  (bind (_x _y) (Class|Arena|GetGridSize))
  (Components|Timeline|SetPlayRate (Variables|Default|GetTimeline_0) (CallFunction|GetAnimationSpeed))
  (for _index (range 0 _x)
    (for _index_2 (range 0 _y)
      (Class|InstancedStaticMeshComponent|AddInstanceWorldSpace (Variables|Default|GetInstancedStaticMesh1) (Math|Transform|MakeTransform (Class|Arena|GetCellLocation (Math|Vector2D|MakeVector2D (Math|Conversions|ToFloat(Integer) _index) (Math|Conversions|ToFloat(Integer) _index_2))) "0, 0, 0" "1,1,1")))))

(event Collision|EventActorBeginOverlap
  (params (OtherActor :type Actor%20Object%20Reference)))

(event EventTick
  (params (DeltaSeconds :type Float%20%28single-precision%29)))

(event EventShowDiceRoll
  (params (Unit :type Unit%20Object%20Reference) (DiceResults :type Integer) (DiceBonus :type Integer) (Phase :type ECombatState%20Enum :default "EInvalid"))
  (bind _returnvalue (Transformation|GetActorLocation Unit))
  (bind _returnvalue_2 (Game|SpawnActorfromClass "/Game/Blueprints/Gameplay/BP_Dice.BP_Dice_C" (Math|Transform|MakeTransform _returnvalue (Math|Rotator|FindLookatRotation (+ _returnvalue "0, 0,50.000000") (Camera|GetCameraLocation (Variables|/Script/Engine.PlayerController|GetPlayerCameraManager (Game|GetPlayerController 0)))) "1,1,1") "Undefined" 0 DiceResults 0))
  (Game|BindEventtoOnDestroyed _returnvalue_2 (delegate Custom|OnDiceFinished))
  (Utilities|Array|Add (Variables|Default|GetActiveDices) _returnvalue_2))

(event EventOnShowMovementRange
  (params (Coords :type Array%20of%20Vector%202D%20Structures))
  (bind _instancedstaticmesh1 (Variables|Default|GetInstancedStaticMesh1))
  (for _array_element Coords
    (Utilities|FlowControl|Sequence
      (:then_0
        (for _array_element_2 (Class|InstancedStaticMeshComponent|GetInstancesOverlappingSphere _instancedstaticmesh1 (Class|Arena|GetCellLocation _array_element) 1.0 true)
          (Class|InstancedStaticMeshComponent|RemoveInstance _instancedstaticmesh1 _array_element_2)))
      (:then_1
        (Class|InstancedStaticMeshComponent|AddInstanceWorldSpace (Variables|Default|GetInstancedStaticMesh2) (Math|Transform|MakeTransform (Class|Arena|GetCellLocation _array_element) "0, 0, 0" "1,1,1"))))))

(event EventOnClearMovementRange
  (params (Coords :type Array%20of%20Vector%202D%20Structures))
  (for _array_element Coords
    (Utilities|FlowControl|Sequence
      (:then_0
        (for _array_element_2 (Class|InstancedStaticMeshComponent|GetInstancesOverlappingSphere (Variables|Default|GetInstancedStaticMesh2) (Class|Arena|GetCellLocation _array_element) 1.0 true)
          (Class|InstancedStaticMeshComponent|RemoveInstance (Variables|Default|GetInstancedStaticMesh2) _array_element_2)))
      (:then_1
        (Class|InstancedStaticMeshComponent|AddInstanceWorldSpace (Variables|Default|GetInstancedStaticMesh1) (Math|Transform|MakeTransform (Class|Arena|GetCellLocation _array_element) "0, 0, 0" "1,1,1"))))))

(event EventExecuteMovement
  (params (Action :type Combat%20Action%20Structure%20%28by%20ref%29))
  (bind (_type _source _targets) (Utilities|Struct|BreakCombatAction Action))
  (bind _outunit (Class|Arena|GetUnitatCell _source))
  (bind _returnvalue (Game|SpawnActorfromClass "/Game/Blueprints/Misc/BP_MovementDummy.BP_MovementDummy_C" (Math|Transform|MakeTransform (Transformation|GetActorLocation _outunit) "0, 0, 0" "1,1,1") "Undefined" 0 0))
  (Transformation|AttachActorToActor _outunit _returnvalue "None" "KeepWorld" "KeepWorld" "KeepWorld" true)
  (bind (_direction _newtrack_0 _newtrack_1) (Timeline|Timeline_0 PlayFromStart)
    (:Update
      (Transformation|SetActorLocation _returnvalue (Math|Vector|MakeVector (.X (Math|Vector|BreakVector (Math|Vector|Lerp(Vector) (Transformation|GetActorLocation _outunit) (Class|Arena|GetCellLocation (Utilities|Array|Get(acopy) _targets)) _newtrack_0))) (.Y (Math|Vector|BreakVector (Math|Vector|Lerp(Vector) (Transformation|GetActorLocation _outunit) (Class|Arena|GetCellLocation (Utilities|Array|Get(acopy) _targets)) _newtrack_0))) (+ (.Z (Math|Vector|BreakVector (Math|Vector|Lerp(Vector) (Transformation|GetActorLocation _outunit) (Class|Arena|GetCellLocation (Utilities|Array|Get(acopy) _targets)) _newtrack_0))) _newtrack_1)) false false))
    (:Finished
      (Transformation|DetachFromActor _outunit "KeepWorld" "KeepWorld" "KeepWorld")
      (Utilities|FlowControl|Delay 0.3)
      (Class|Arena|OnActionFinished Action))))

(event EventOnPreReady
  (|CallParentFunction)
  (Class|ArcanaController|OnTransitiontoCombatFinished (.AsBP%20User%20Controller (Utilities|Casting|CastToBP_UserController (Game|GetPlayerController 0)))))

(event EventExecuteMoveAttack
  (params (Action :type Combat%20Action%20Structure%20%28by%20ref%29))
  (bind (_type _source _targets) (Utilities|Struct|BreakCombatAction Action))
  (bind _outunit (Class|Arena|GetUnitatCell _source))
  (bind _returnvalue (Game|SpawnActorfromClass "/Game/Blueprints/Misc/BP_MovementDummy.BP_MovementDummy_C" (Math|Transform|MakeTransform (Transformation|GetActorLocation _outunit) "0, 0, 0" "1,1,1") "Undefined" 0 0))
  (Transformation|AttachActorToActor _outunit _returnvalue "None" "KeepWorld" "KeepWorld" "KeepWorld" true)
  (bind (_direction _newtrack_0 _newtrack_1) (Timeline|Timeline_1 PlayFromStart)
    (:Update
      (Transformation|SetActorLocation _returnvalue (Math|Vector|MakeVector (.X (Math|Vector|BreakVector (Math|Vector|Lerp(Vector) (Transformation|GetActorLocation _outunit) (Class|Arena|GetCellLocation (Utilities|Array|Get(acopy) _targets)) _newtrack_0))) (.Y (Math|Vector|BreakVector (Math|Vector|Lerp(Vector) (Transformation|GetActorLocation _outunit) (Class|Arena|GetCellLocation (Utilities|Array|Get(acopy) _targets)) _newtrack_0))) (+ (.Z (Math|Vector|BreakVector (Math|Vector|Lerp(Vector) (Transformation|GetActorLocation _outunit) (Class|Arena|GetCellLocation (Utilities|Array|Get(acopy) _targets)) _newtrack_0))) _newtrack_1)) false false))
    (:Finished
      (Transformation|DetachFromActor _outunit "KeepWorld" "KeepWorld" "KeepWorld")
      (Utilities|FlowControl|Delay 0.3)
      (Class|Arena|OnActionFinished Action))))

(fn ConstructionScript
  (bind _arenasize (Variables|Pebble|GetArenaSize))
  (Utilities|FlowControl|Sequence
    (:then_0
      (for _index (range 0 (Math|Float|Truncate (.x _arenasize)))
        (for _index_2 (range 0 (Math|Float|Truncate (.y _arenasize)))
          (Class|InstancedStaticMeshComponent|AddInstanceWorldSpace (Variables|Default|GetInstancedStaticMesh) (Math|Transform|MakeTransform (Utilities|MakeLocforMesh _index _index_2) (Utilities|MakeRotforMesh) (Math|Conversions|ToVector(Float) (Variables|Pebble|GetTileScale)))))))))

(fn DrawDebug)

(fn NewFunction0)