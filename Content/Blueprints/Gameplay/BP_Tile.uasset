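; BP_Tile is a grid tile actor that shows hover feedback and plays a fog-clearing reveal.
; On cursor hover, it asks the grid subsystem whether the player can travel to it and sets one of two custom depth stencil values on its mesh, clearing it when the cursor leaves.
; OnReveal runs a timeline that scales the temporary fog component, then destroys it when finished.
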(event OnBeginCursorOver(MeshComp)
  (params (TouchedComponent :type Primitive%20Component%20Object%20Reference))
  (Rendering|SetCustomDepthStencilValue (Variables|Default|GetMeshComp) (Math|Integer|SelectInt 253 254 (Class|GridSubsystem|CanPlayerTraveltoTile (Subsystems|GetGridSubsystem) self))))

(event OnEndCursorOver(MeshComp)
  (params (TouchedComponent :type Primitive%20Component%20Object%20Reference))
  (Rendering|SetCustomDepthStencilValue (Variables|Default|GetMeshComp) 0))

(event EventBeginPlay)

(event Collision|EventActorBeginOverlap
  (params (OtherActor :type Actor%20Object%20Reference)))

(event EventTick
  (params (DeltaSeconds :type Float%20%28single-precision%29)))

(event EventOnReveal
  (bind _tempfogcomp (Variables|Default|GetTempFogComp))
  (bind _newtrack_0 (Timeline|Timeline_0 PlayFromStart)
    (:Update
      (Transformation|SetWorldScale3D _tempfogcomp (Math|Conversions|ToVector(Float) _newtrack_0)))
    (:Finished
      (Components|DestroyComponent _tempfogcomp))))

(fn ConstructionScript)