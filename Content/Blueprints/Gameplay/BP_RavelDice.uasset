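; BP_RavelDice is a physics-simulated die that spawns with a random right-angle rotation and plays a roll sound shortly after.
; When the mesh's physics body sleeps, it passes its roll type and value to the GameMode, then freezes.
; A timeline animates its scale, spawns an arcane death effect and destroys it.
; Rolls below the hit value also spawn a miss effect.
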(event OnClicked(DiceMesh)
  (params (TouchedComponent :type Primitive%20Component%20Object%20Reference) (ButtonPressed :type Key%20Structure)))

(event OnComponentSleep(DiceMesh)
  (params (SleepingComponent :type Primitive%20Component%20Object%20Reference) (BoneName :type Name :default "None"))
  (bind _dicemesh (Variables|Default|GetDiceMesh))
  (bind _rolledvalue (Variables|Default|GetRolledValue))
  (Utilities|FlowControl|Delay 0.01)
  (Utilities|FlowControl|Sequence
    (:then_0
      (Default|CallOnDiceRoll (Variables|Default|GetGameMode) (Variables|Default|GetRollType) _rolledvalue))
    (:then_1
      (Physics|SetSimulatePhysics _dicemesh false)
      (Collision|SetCollisionEnabled _dicemesh "NoCollision")
      (Utilities|FlowControl|Delay (Math|Random|RandomFloatinRange 0.0 0.3))
      (bind _newtrack_0 (Timeline|Timeline_0 PlayFromStart)
        (:Update
          (Transformation|SetActorScale3D (* _newtrack_0 0.8)))
        (:Finished
          (Actor|DestroyActor :!label _label))
        (:Spawn
          (Effects|SpawnEmitteratLocation "/Game/Prototype/Particles/PS_ArcaneDeath.PS_ArcaneDeath" (Transformation|GetActorLocation))
          (goto _label))))
    (:then_2
      (if (< _rolledvalue (Variables|Default|GetHitValue))
        (Effects|SpawnEmitteratLocation "/Game/Particles/PS_Miss.PS_Miss" (Transformation|GetActorLocation))))))

(event EventBeginPlay
  (bind _dicemesh (Variables|Default|GetDiceMesh))
  (Physics|SetSimulatePhysics (Variables|Default|GetDiceMesh) false)
  (Collision|SetCollisionEnabled _dicemesh "NoCollision")
  (Utilities|FlowControl|Delay 0.01)
  (Collision|SetCollisionEnabled _dicemesh "QueryAndPhysics")
  (Physics|SetSimulatePhysics (Variables|Default|GetDiceMesh) true)
  (Utilities|FlowControl|Delay 0.3)
  (Audio|PlaySound2D "/Game/Sounds/dice_w.dice_w" 1.0 1.0 0.0 0 0))

(event Collision|EventActorBeginOverlap
  (params (OtherActor :type Actor%20Object%20Reference)))

(event EventTick
  (params (DeltaSeconds :type Float%20%28single-precision%29)))

(fn ConstructionScript
  (Transformation|SetActorRotation (Math|Rotator|MakeRotator (* (Math|Random|RandomInteger 6) 9e+01) (* (Math|Random|RandomInteger 6) 9e+01) (* (Math|Random|RandomInteger 6) 9e+01))))