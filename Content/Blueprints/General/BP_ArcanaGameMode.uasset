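; Game mode for Arcana that sets up the city actor and player pawn on begin play and animates party movement.
; Movement timeline play rate comes from the animation speed setting, and pawn initialization follows city setup after a tiny delay.
; OnMoveParty attaches party members to a temporary dummy, which a timeline lerps from start to finish with an added height curve.
; When it finishes, members detach and the dummy is destroyed.
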(event EventBeginPlay
  (|CallParentFunction)
  (Components|Timeline|SetPlayRate (Variables|Default|GetTimeline_0) (CallFunction|GetAnimationSpeed))
  (bind _returnvalue (Actor|GetActorOfClass "/Game/Blueprints/Gameplay/BP_DebugCity.BP_DebugCity_C"))
  (Class|ArcanaBoardGameModeBase|InitCityActor _returnvalue)
  (Utilities|FlowControl|Delay 1e-05)
  (Class|ArcanaBoardGameModeBase|InitPlayerPawn "(X=0.000000,Y=0.000000)"))

(event EventTick
  (params (DeltaSeconds :type Float%20%28single-precision%29)))

(event EventOnMoveParty
  (params (Party :type Party%20Object%20Reference) (Start :type Tile%20Object%20Reference) (Finish :type Tile%20Object%20Reference))
  (bind _returnvalue (Transformation|GetActorLocation Start))
  (bind _returnvalue_2 (Class|Party|GetMembers Party))
  (bind _returnvalue_3 (Game|SpawnActorfromClass "/Game/Blueprints/Misc/BP_MovementDummy.BP_MovementDummy_C" (Math|Transform|MakeTransform _returnvalue "0, 0, 0" "1,1,1") "Undefined" 0 0))
  (for _array_element _returnvalue_2
    (Transformation|AttachActorToActor _array_element _returnvalue_3 "None" "KeepWorld" "KeepWorld" "KeepWorld" true))
  (bind (_direction _newtrack_0 _newtrack_1) (Timeline|Timeline_0 PlayFromStart)
    (:Update
      (Transformation|SetActorLocation _returnvalue_3 (Math|Vector|MakeVector (.X (Math|Vector|BreakVector (Math|Vector|Lerp(Vector) _returnvalue (Transformation|GetActorLocation Finish) _newtrack_0))) (.Y (Math|Vector|BreakVector (Math|Vector|Lerp(Vector) _returnvalue (Transformation|GetActorLocation Finish) _newtrack_0))) (+ (.Z (Math|Vector|BreakVector (Math|Vector|Lerp(Vector) _returnvalue (Transformation|GetActorLocation Finish) _newtrack_0))) _newtrack_1)) false false))
    (:Finished
      (bind _returnvalue_4 (Class|Party|GetMembers Party))
      (for _array_element_2 _returnvalue_4
        (Transformation|DetachFromActor _array_element_2 "KeepWorld" "KeepWorld" "KeepWorld"))
      (Actor|DestroyActor _returnvalue_3))))

(fn ConstructionScript)