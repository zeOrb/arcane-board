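; Player controller that handles the transition into combat and a mouse-following cell marker on the battle grid.
; On transition it plays the TransitionToCombat sequence, blends to the supplied camera after a delay, then spawns a movable plane mesh with a battle-cell material.
; Each tick moves that marker to the plane-projected mouse position, snapped to the grid and within a region, at a fixed height.
; The transition-finished event only calls its parent.
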(event EventBeginPlay)

(event EventTick
  (params (DeltaSeconds :type Float%20%28single-precision%29))
  (bind _returnvalue (Class|ArcanaController|GetMouseProjectedtoPlane "-0.000000,0.000000,-64.248970"))
  (bind _returnvalue_2 (Class|ArcanaController|SnaptoGrid _returnvalue))
  (bind _returnvalue_3 (Class|ArcanaController|SnapWithinRegion _returnvalue_2))
  (bind (_x _y) (Math|Vector|BreakVector _returnvalue_3))
  (if (Utilities|IsValid (Variables|Default|GetNewVar_1))
    (Transformation|SetActorLocation (Variables|Default|GetNewVar_1) (Class|ArcanaController|SnaptoGrid (Math|Vector|MakeVector _x _y -60.24897)) false false)))

(event EventOnBeginTransitiontoCombat
  (params (CameraActor :type Actor%20Object%20Reference))
  (bind _returnvalue (Sequencer|Player|CreateLevelSequencePlayer "/Game/TransitionToCombat.TransitionToCombat"))
  (Utilities|FlowControl|Sequence
    (:then_0
      (Sequencer|Player|Play _returnvalue :!class /Script/MovieScene.MovieSceneSequencePlayer))
    (:then_1
      (Utilities|FlowControl|Delay 0.6)
      (Game|Player|SetViewTargetwithBlend CameraActor 0.1 "VTBlend_EaseIn" 1.0 false)
      (Utilities|FlowControl|Delay 1.0)
      (bind _returnvalue_2 (Game|SpawnActorfromClass "/Script/Engine.StaticMeshActor" (Math|Transform|MakeTransform "0, 0, 0" "0, 0, 0" "1,1,1") "Undefined" 0 0))
      (Transformation|SetMobility _returnvalue_2 "Movable")
      (Variables|Default|SetNewVar_1 _returnvalue_2)
      (Components|StaticMesh|SetStaticMesh (Variables|/Script/Engine.StaticMeshActor|GetStaticMeshComponent _returnvalue_2) "/Game/Meshes/Misc/SM_CombatPlaneSmall.SM_CombatPlaneSmall")
      (Rendering|Material|SetMaterial (Variables|/Script/Engine.StaticMeshActor|GetStaticMeshComponent _returnvalue_2) 0 "/Game/Materials/VisualEffects/M_BattleCell_Inst.M_BattleCell_Inst"))))

(event EventOnTransitiontoCombatFinished
  (|CallParentFunction))

(fn ConstructionScript)