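; BP_TestingGenerator is a test actor that spawns a BP_TestingProjectile at its own location every tick.
; Each projectile launches in a random direction within a narrow cone around the Arrow component's forward vector, with random uniform scale and speed.
; Direction draws from a random stream while scale and speed use global random, and an Objects counter tracks the total spawned.
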(event EventBeginPlay)

(event Collision|EventActorBeginOverlap
  (params (OtherActor :type Actor%20Object%20Reference)))

(event EventTick
  (params (DeltaSeconds :type Float%20%28single-precision%29))
  (Game|SpawnActorfromClass "/Game/Testing/Blueprints/BP_TestingProjectile.BP_TestingProjectile_C" (Math|Transform|MakeTransform (Transformation|GetActorLocation) (Math|Rotator|MakeRotfromX (Math|Random|RandomUnitVectorinConeinDegreesfromStream (Math|Vector|GetForwardVector (Transformation|GetWorldRotation (Variables|Default|GetArrow))) 15.0 (Variables|Default|GetRandomStream))) (Math|Conversions|ToVector(Float) (Math|Random|RandomFloatinRange 0.5 1.5))) "AlwaysSpawn" 0 (Math|Random|RandomFloatinRange 5e+02 1e+03) 0)
  (Math|Integer|IncrementInt (Variables|Default|GetObjects)))

(fn ConstructionScript)